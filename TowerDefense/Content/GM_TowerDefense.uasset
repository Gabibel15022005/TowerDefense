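; Tower defense game mode that spawns and possesses the camera pawn, starts the player controller and runs enemy waves.
; PopulateMap reads the wave's row from DT_WaveDetails into a map of remaining counts per enemy class and totals them.
; A looping timer has a random BP_EnemySpawn spawn a random enemy type that still has count left.
; Once none remain to spawn or alive, it loads the next wave.
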(event `self.ReceiveBeginPlay`
  (`self.PlayerSetup`)
  (bind _outactors (`GameplayStatics.GetAllActorsOfClass` "/Game/GameObjects/GoalOfEnemy/BP_EnemySpawn.BP_EnemySpawn_C"))
  (set `self.Out Actors` _outactors)
  (`KismetSystemLibrary.K2_SetTimerDelegate` (delegate `ActivateSpawner`) 2.0 true)
  (`self.PopulateMap` (`self.WaveNb`)))

(event `ActivateSpawner`
  (bind _out_actors (`self.Out Actors`))
  (if (> (`self.EnemiesNb`) 0)
    (bind _enemy_chosen (`self.ChooseEnemy`))
    (`/Game/GameObjects/GoalOfEnemy/BP_EnemySpawn.SpawnEnemyFunction` (`|GetArrayItem` _out_actors (`KismetMathLibrary.RandomIntegerInRange` 0 (- (`KismetArrayLibrary.Array_Length` _out_actors) 1))) _enemy_chosen)
    (else
      (bind _outactors (`GameplayStatics.GetAllActorsOfClass` "/Game/GameObjects/TestEnemy/BP_TestEnemyParent.BP_TestEnemyParent_C"))
      (if (<= (`KismetArrayLibrary.Array_Length` _outactors) 0)
        (bind _result (`/Engine/EditorBlueprintResources/StandardMacros.IncrementInt` (`self.WaveNb`))
          (:`  `
            (`self.PopulateMap` _result)))))))

(event `PlayerSetup`
  (bind _returnvalue (`GameplayStatics.GetPlayerController` 0))
  ;[1 0.009772 0.02658 0.5] Start function
  (bind _returnvalue_2 (`|SpawnActorFromClass` (`self.DefaultActor`) (`KismetMathLibrary.MakeTransform` (0.0 0.0 2.0)) "AdjustIfPossibleButAlwaysSpawn" "MultiplyWithRoot" null null))
  (bind _asc_cam (cast `/Game/Player/C_Cam` _returnvalue_2)
    (:`then`
      (`Controller.Possess` _returnvalue _asc_cam)
      (bind _aspc_tower_defense (cast `/Game/Player/PC_TowerDefense` _returnvalue))
      (`/Game/Player/PC_TowerDefense.Start` _aspc_tower_defense))
    (:`CastFailed`
      (`KismetSystemLibrary.PrintString` "Cast failed in GM_TowerDefense" true true (struct :`R` 1.0 :`G` 0.044108 :`A` 1.0) 5.0))))

(fn `ChooseEnemy`
  (returns (`Enemy Chosen` :type "/Game/GameObjects/TestEnemy/BP_TestEnemyParent Class Reference"))
  (bind _keys (`BlueprintMapLibrary.Map_Keys` (`self.EnemyList`) :!label _label))
  (bind _output_get (set `self.Chose Enemy` (`|GetArrayItem` _keys (`KismetMathLibrary.RandomInteger` (`KismetArrayLibrary.Array_Length` _keys)))))
  (bind _value (`BlueprintMapLibrary.Map_Find` (`self.EnemyList`) _output_get))
  (set `self.NewVar` _value)
  (if (> _value 0)
    (`BlueprintMapLibrary.Map_Add` (`self.EnemyList`) (`self.Chose Enemy`) (- (`self.NewVar`) 1))
    (`/Engine/EditorBlueprintResources/StandardMacros.DecrementInt` (`self.EnemiesNb`)
      (:`  `
        (return (`self.Chose Enemy`))))
    (else
      (goto _label))))

(fn `PopulateMap`
  (params (WaveNumber :type Integer))
  (bind _returnvalue (`|GetDataTableRow` "/Game/GameObjects/TestEnemy/DT_WaveDetails.DT_WaveDetails" (`KismetStringLibrary.Conv_StringToName` (`KismetStringLibrary.Conv_IntToString` WaveNumber)))
    (:`then`
      (bind _output_get (set `self.EnemyList` (`|MakeMap` "/Game/GameObjects/TestEnemy/C_TestEnemy.C_TestEnemy_C" (break `/Game/GameObjects/TestEnemy/S_WaveDetails` _returnvalue) "/Game/GameObjects/TestEnemy/C_TestEnemySmall.C_TestEnemySmall_C" (`.BasicSmall_4_474D91BB4C1A81B3B7F196B169818B9D` (break `/Game/GameObjects/TestEnemy/S_WaveDetails` _returnvalue)) "/Game/GameObjects/TestEnemy/C_TestEnemyBig.C_TestEnemyBig_C" (`.BasicBig_6_DEB9858547495742F33FC292DDE0BCB8` (break `/Game/GameObjects/TestEnemy/S_WaveDetails` _returnvalue)) :!type "/Game/GameObjects/TestEnemy/BP_TestEnemyParent Class Reference")))
      (bind _values (`BlueprintMapLibrary.Map_Values` _output_get))
      (for _array_element _values
        (set `self.EnemiesNb` (+ _array_element (`self.EnemiesNb`)))))))

(fn `UserConstructionScript`)