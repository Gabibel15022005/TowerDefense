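; Boid manager that steers tower-defense enemies along a shared waypoint list as a flock, updated every Tick.
; Each boid sums separation, alignment and cohesion from neighbors within a radius, checked pairwise on the horizontal plane.
; These blend by weight with the direction to the next navmesh path point, setting the boid's velocity and rotation.
; Boids reaching the last waypoint are destroyed and decrement the game mode's enemy total.
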(event `self.ReceiveTick`
  (params (DeltaSeconds :type "Float (single-precision)"))
  (for _array_element (`self.Waypoints`)
    (`KismetSystemLibrary.DrawDebugSphere` (`self.K2_GetActorLocation` _array_element) (`self.WaypointCheckRadius`) 8))
  (`self.UpdateBoids` DeltaSeconds))

(fn `AddAlignement`
  (params (Neighbor :type "/Game/GameObjects/TestEnemy/BP_TestEnemyParent Object Reference"))
  (returns (VectorToAdd :type "Vector Structure"))
  (bind (_velocity_x _velocity_y) (`KismetMathLibrary.BreakVector` (`MovementComponent.Velocity` (`Character.CharacterMovement` Neighbor))))
  (return (`KismetMathLibrary.MakeVector` _velocity_x _velocity_y)))

(fn `AddCohesion`
  (params (Neighbor :type "/Game/GameObjects/TestEnemy/BP_TestEnemyParent Object Reference") (Actual :type "/Game/GameObjects/TestEnemy/BP_TestEnemyParent Object Reference"))
  (returns (`Vector To Add` :type "Vector Structure"))
  (bind (_returnvalue_x _returnvalue_y) (`KismetMathLibrary.BreakVector` (`self.K2_GetActorLocation` Actual)))
  (bind (_returnvalue_x_2 _returnvalue_y_2) (`KismetMathLibrary.BreakVector` (`self.K2_GetActorLocation` Neighbor)))
  (return (- (`KismetMathLibrary.MakeVector` _returnvalue_x_2 _returnvalue_y_2) (`KismetMathLibrary.MakeVector` _returnvalue_x _returnvalue_y))))

(fn `AddSeparation`
  (params (Actual :type "Actor Object Reference") (Neighbor :type "Actor Object Reference"))
  (returns (VectorToAdd :type "Vector Structure"))
  (locals (Distance :type "Float (double-precision)") (DirectionAway :type "Vector Structure") (Normalized :type "Vector Structure") (Force :type "Vector Structure"))
  (bind (_returnvalue_x _returnvalue_y) (`KismetMathLibrary.BreakVector` (`self.K2_GetActorLocation` Neighbor)))
  (bind (_returnvalue_x_2 _returnvalue_y_2) (`KismetMathLibrary.BreakVector` (`self.K2_GetActorLocation` Actual)))
  (bind _output_get (set `local.DirectionAway` (- (`KismetMathLibrary.MakeVector` _returnvalue_x_2 _returnvalue_y_2) (`KismetMathLibrary.MakeVector` _returnvalue_x _returnvalue_y))))
  (bind _output_get_2 (set `local.Distance` (`KismetMathLibrary.VSize` _output_get)))
  (if (== _output_get_2 0.0)
    (return (0.0 0.0 0.0))
    (else
      (bind _output_get_3 (set `local.Normalized` (`KismetMathLibrary.Normal` (`local.DirectionAway`))))
      (bind _output_get_4 (set `local.Force` (/ _output_get_3 (`local.Distance`))))
      (return _output_get_4))))

(fn `ApplyVelocityToBoid`
  (params (SeparationSum :type "Vector Structure") (AlignementSum :type "Vector Structure") (CohesionSum :type "Vector Structure") (`Direction To Waypoint` :type "Vector Structure") (Count :type Integer) (Boid :type "/Game/GameObjects/TestEnemy/BP_TestEnemyParent Object Reference") (DeltaTime :type "Float (double-precision)"))
  (returns (FinalForceRef :type "Vector Structure"))
  (locals (SeparationForce :type "Vector Structure") (AlignementForce :type "Vector Structure") (CohesionForce :type "Vector Structure") (FinalForce :type "Vector Structure"))
  (bind _boid (`local.Boid`))
  (bind (_returnvalue_x _returnvalue_y) (`KismetMathLibrary.BreakVector` (+ (* (`self.Separation Weight`) (`local.SeparationForce`)) (* (`self.Alignement Weight`) (`local.AlignementForce`)) (* (`self.Cohesion Weight`) (`local.CohesionForce`)) (* (`self.Target Weight`) (`local.Direction To Waypoint`)))))
  (if (> Count 0)
    (set `local.SeparationForce` (`KismetMathLibrary.Normal` (/ (`local.SeparationSum`) (`local.Count`))))
    (set `local.AlignementForce` (`KismetMathLibrary.Normal` (/ (`local.AlignementSum`) (`local.Count`))))
    (set `local.CohesionForce` (`KismetMathLibrary.Normal` (/ (`local.CohesionSum`) (`local.Count`))))
    (else
      (set `local.SeparationForce` (0.0 0.0 0.0))
      (set `local.AlignementForce` (0.0 0.0 0.0))
      (set `local.CohesionForce` (0.0 0.0 0.0))))
  (bind _output_get (set `local.FinalForce` (`KismetMathLibrary.MakeVector` _returnvalue_x _returnvalue_y)))
  (bind _returnvalue (+ (`KismetMathLibrary.Normal` (`MovementComponent.Velocity` (`Character.CharacterMovement` (`local.Boid`)))) (* _output_get (`self.FinalForce Weight`) (`local.DeltaTime`))))
  (set `/Game/GameObjects/TestEnemy/BP_TestEnemyParent.Velocity` _returnvalue _boid)
  (set `/Game/GameObjects/TestEnemy/BP_TestEnemyParent.Rotation` (`KismetMathLibrary.MakeRotFromX` _returnvalue) _boid)
  (return (`local.FinalForce`)))

(fn `CalculateDirectionToWaypoint`
  (params (Actual :type "/Game/GameObjects/TestEnemy/BP_TestEnemyParent Object Reference"))
  (returns (`Vector Direction` :type "Vector Structure") (Distance :type "Float (double-precision)"))
  (bind _returnvalue (`self.K2_GetActorLocation` Actual))
  (bind _returnvalue_2 (`self.K2_GetActorLocation` (`|GetArrayItem` (`self.Waypoints`) (`/Game/GameObjects/TestEnemy/BP_TestEnemyParent.CurrentWaypoint` Actual))))
  (bind _returnvalue_3 (`KismetMathLibrary.VSize` (- _returnvalue_2 _returnvalue)))
  (bind _returnvalue_4 (`NavigationSystemV1.FindPathToLocationSynchronously` _returnvalue _returnvalue_2 null null))
  (bind _output (`|GetArrayItem` (`NavigationPath.PathPoints` _returnvalue_4) 1))
  (set `/Game/GameObjects/TestEnemy/BP_TestEnemyParent.PathPoint` _output (`local.Actual`))
  (if (== _returnvalue_3 0.0)
    (return (0.0 0.0 0.0) _returnvalue_3)
    (else
      (return (`KismetMathLibrary.Normal` (- _output (`self.K2_GetActorLocation` (`local.Actual`)))) _returnvalue_3))))

(fn `UpdateBoids`
  (params (DeltaTime :type "Float (double-precision)"))
  (locals (Separation :type "Vector Structure") (Alignement :type "Vector Structure") (Cohesion :type "Vector Structure") (NeighborCount :type Integer) (ActualBoid :type "/Game/GameObjects/TestEnemy/BP_TestEnemyParent Object Reference") (ActualNeighbor :type "/Game/GameObjects/TestEnemy/BP_TestEnemyParent Object Reference") (DirectionToWaypoint :type "Vector Structure"))
  (bind _actualboid (`local.ActualBoid`))
  (bind (_returnvalue_x _returnvalue_y _returnvalue_z) (`KismetMathLibrary.BreakVector` (`self.K2_GetActorLocation` (`local.ActualBoid`))))
  (bind (_returnvalue_x_2 _returnvalue_y_2) (`KismetMathLibrary.BreakVector` (`self.K2_GetActorLocation` (`local.ActualNeighbor`))))
  (bind _currentwaypoint (`/Game/GameObjects/TestEnemy/BP_TestEnemyParent.CurrentWaypoint` _actualboid))
  (bind _returnvalue (`KismetMathLibrary.MakeVector` _returnvalue_x_2 _returnvalue_y_2 _returnvalue_z))
  (bind _returnvalue_2 (`KismetMathLibrary.MakeVector` _returnvalue_x _returnvalue_y _returnvalue_z))
  (if (!= (`KismetArrayLibrary.Array_Length` (`self.Waypoints`)) 0)
    (for _array_element (`self.BoidList`)
      (`/Engine/EditorBlueprintResources/StandardMacros.IsValid` _array_element
        (:`Is Valid`
          (set `local.ActualBoid` _array_element)
          ;[1 0.02293 0 0.5] Reset Local Variable Foreach Ennemie
          (set `local.Separation` (0.0 0.0 0.0))
          (set `local.Alignement` (0.0 0.0 0.0))
          (set `local.Cohesion` (0.0 0.0 0.0))
          (set `local.NeighborCount` 0)
          (for _array_element_2 (`self.BoidList`)
            (`/Engine/EditorBlueprintResources/StandardMacros.IsValid` _array_element_2
              (:`Is Valid`
                (if (!= _array_element_2 _array_element)
                  (set `local.ActualNeighbor` _array_element_2)
                  (if (<= (`KismetMathLibrary.Vector_Distance` _returnvalue_2 _returnvalue) (`self.NeighborDetectorRadius`))
                    (`KismetSystemLibrary.DrawDebugLine` _returnvalue_2 _returnvalue (struct :`G` 1.0 :`B` 0.103468 :`A` 1.0) (`self.CheckInterval`) 10.0)
                    (set `local.NeighborCount` (+ (`local.NeighborCount`) 1))
                    ;[1 0.994 0 0.5] Ajouter séparation / alignement / cohesion
                    ;;[0.1364 1 0 0.5] Separation
                    (bind _vectortoadd (`self.AddSeparation` (`local.ActualBoid`) (`local.ActualNeighbor`)))
                    (set `local.Separation` (+ _vectortoadd (`local.Separation`)))
                    ;;[1 0 0.03627 0.5] Alignement
                    (bind _vectortoadd_2 (`self.AddAlignement` (`local.ActualNeighbor`)))
                    (set `local.Alignement` (+ _vectortoadd_2 (`local.Alignement`)))
                    ;;[1 0 0.8983 0.5] Cohesion
                    (bind _vector_to_add (`self.AddCohesion` (`local.ActualNeighbor`) (`local.ActualBoid`)))
                    (set `local.Cohesion` (+ _vector_to_add (`local.Cohesion`))))))))
          ; Donner la nouvelle vélocité en la calculant avec les variables locales
          (bind (_vector_direction _distance) (`self.CalculateDirectionToWaypoint` (`local.ActualBoid`) :!label _label))
          (if (<= _distance (`self.WaypointCheckRadius`))
            (if (< _currentwaypoint (- (`KismetArrayLibrary.Array_Length` (`self.Waypoints`)) 1))
              (set `/Game/GameObjects/TestEnemy/BP_TestEnemyParent.CurrentWaypoint` (+ _currentwaypoint 1) _actualboid)
              (goto _label)
              (else
                (`KismetSystemLibrary.PrintString` "Reached last Waypoint" true true (struct :`R` 0.207244 :`G` 1.0 :`A` 1.0))
                (`self.K2_DestroyActor` (`local.ActualBoid`))
                (bind _asgm_tower_defense (cast `/Game/GM_TowerDefense` (`GameplayStatics.GetGameMode`)))
                (set `/Game/GM_TowerDefense.TotalEnemies` (- (`/Game/GM_TowerDefense.TotalEnemies` _asgm_tower_defense) 1) _asgm_tower_defense)))
            (else
              (set `local.DirectionToWaypoint` _vector_direction)
              (`self.ApplyVelocityToBoid` (`local.Separation`) (`local.Alignement`) (`local.Cohesion`) (`local.DirectionToWaypoint`) (`local.NeighborCount`) (`local.ActualBoid`) (`local.DeltaTime`))
              ;;[1 0 0.7538 0.5] Give Value For Debug*
              (set `/Game/GameObjects/TestEnemy/BP_TestEnemyParent.WaypointLocation` (`self.K2_GetActorLocation` (`|GetArrayItem` (`self.Waypoints`) (`/Game/GameObjects/TestEnemy/BP_TestEnemyParent.CurrentWaypoint` (`local.ActualBoid`)))) (`local.ActualBoid`))
              (set `/Game/GameObjects/TestEnemy/BP_TestEnemyParent.DirectionToWaypoint` (+ (`self.K2_GetActorLocation` (`local.ActualBoid`)) (* (`local.DirectionToWaypoint`) 200.0)) (`local.ActualBoid`)))))))
    (else
      (`KismetSystemLibrary.PrintString` "No Waypoint found"))))

(fn `UserConstructionScript`)