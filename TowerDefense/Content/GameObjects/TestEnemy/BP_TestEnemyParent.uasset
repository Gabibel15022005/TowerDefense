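; Parent test enemy character that moves as a boid agent, registering itself with the first BP_BoidManager found on BeginPlay and applying its walk speed.
; Each tick it feeds its Velocity variable into movement input and smoothly interpolates its rotation toward a target Rotation; neither value is computed in this graph.
; Tick also draws debug shapes for the waypoint, waypoint direction and current path point.
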(event `self.ReceiveBeginPlay`
  (bind _outactors (`GameplayStatics.GetAllActorsOfClass` "/Game/GameObjects/TestEnemy/BP_BoidManager.BP_BoidManager_C"))
  (`KismetArrayLibrary.Array_Add` (`/Game/GameObjects/TestEnemy/BP_BoidManager.BoidList` (`|GetArrayItem` _outactors)) self)
  (set `CharacterMovementComponent.MaxWalkSpeed` (`self.Max Walk Speed`) (`self.CharacterMovement`)))

(event `self.ReceiveTick`
  (params (DeltaSeconds :type "Float (single-precision)"))
  (`self.AddMovementInput` (`self.Velocity`))
  (`self.K2_SetActorRotation` (`KismetMathLibrary.RInterpTo` (`self.K2_GetActorRotation`) (`self.Rotation`) DeltaSeconds (`self.Rotation Speed`)))
  (`KismetSystemLibrary.DrawDebugLine` (`self.K2_GetActorLocation`) (`self.WaypointLocation`) (struct :`R` 1.0 :`G` 0.081366 :`A` 1.0) 0.0 1.0)
  (`KismetSystemLibrary.DrawDebugArrow` (`self.K2_GetActorLocation`) (`self.DirectionToWaypoint`) 0.0 (struct :`R` 1.0 :`B` 0.955077 :`A` 1.0) 0.0 10.0)
  (`KismetSystemLibrary.DrawDebugSphere` (`self.PathPoint`) 50.0 6 (struct :`G` 0.129103 :`B` 1.0 :`A` 1.0) 0.0 1.0))

(fn `UserConstructionScript`)