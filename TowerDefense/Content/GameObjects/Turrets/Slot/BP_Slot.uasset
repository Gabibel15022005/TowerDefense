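; BP_Slot is a turret slot actor that gives visual feedback for mouse interaction.
; Cursor and click events on its Slot component swap the material in the first slot between mouse-over, mouse-out and clicked looks, returning to mouse-over on release.
; It holds no turret placement logic; BeginPlay, overlap, Tick and the construction script are empty.
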(event `self.Slot.OnBeginCursorOver`
  (params (TouchedComponent :type "PrimitiveComponent Object Reference"))
  (`PrimitiveComponent.SetMaterial` (`self.Slot`) 0 "/Game/GameObjects/Turrets/MaterialSlot/M_MouseOver.M_MouseOver"))

(event `self.Slot.OnEndCursorOver`
  (params (TouchedComponent :type "PrimitiveComponent Object Reference"))
  (`PrimitiveComponent.SetMaterial` (`self.Slot`) 0 "/Game/GameObjects/Turrets/MaterialSlot/M_MouseOut.M_MouseOut"))

(event `self.Slot.OnClicked`
  (params (TouchedComponent :type "PrimitiveComponent Object Reference") (ButtonPressed :type "Key Structure"))
  (`PrimitiveComponent.SetMaterial` (`self.Slot`) 0 "/Game/GameObjects/Turrets/MaterialSlot/M_MouseClicked.M_MouseClicked"))

(event `self.Slot.OnReleased`
  (params (TouchedComponent :type "PrimitiveComponent Object Reference") (ButtonReleased :type "Key Structure"))
  (`PrimitiveComponent.SetMaterial` (`self.Slot`) 0 "/Game/GameObjects/Turrets/MaterialSlot/M_MouseOver.M_MouseOver"))

(fn `UserConstructionScript`)