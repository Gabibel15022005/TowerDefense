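; Player controller for the tower defense camera, driving a C_Cam pawn with speeds and zoom limits stored on that pawn.
; Start, called by GM_Demo, caches the pawn, adds the movement input mapping and sets Game and UI input with the mouse locked.
; Enhanced Input moves the camera by local offsets without sweep, with a hold-to-accelerate speed switch.
; Mouse wheel key events change the spring arm length, clamped between the zoom limits.
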(event `Start`
  (bind _as_c_cam (`self.As C Cam`))
  ;[1 0 0.119 0.5] Called by GM_Demo on start
  (bind _asc_cam (cast `/Game/Player/C_Cam` (`GameplayStatics.GetPlayerCharacter` 0)))
  (set `self.As C Cam` _asc_cam)
  (`EnhancedInputSubsystemInterface.AddMappingContext` (pcsubsystem `EnhancedInputLocalPlayerSubsystem` self) "/Game/Inputs/Movements/IMC_Movements.IMC_Movements" 0 (struct))
  (`WidgetBlueprintLibrary.SetInputMode_GameAndUIEx` self null "LockAlways" false)
  (set `/Game/Player/C_Cam.CurrentSpeed` (`/Game/Player/C_Cam.BaseSpeed` _as_c_cam) _as_c_cam))

(event `EnhancedInput|/Game/Inputs/Movements/IA_ForwardBackward`
  (params (ActionValue :type "Float (double-precision)") (ElapsedSeconds :type "Float (double-precision)") (TriggeredSeconds :type "Float (double-precision)") (InputAction :type "InputAction Object Reference" :default "/Game/Inputs/Movements/IA_ForwardBackward.IA_ForwardBackward"))
  (bind _as_c_cam (`self.As C Cam`))
  ;[0.01896 0 1 0.5] Movement
  (:`Triggered`
    (`self.K2_AddActorLocalOffset` _as_c_cam (`KismetMathLibrary.MakeVector` (* (`/Game/Player/C_Cam.CurrentSpeed` _as_c_cam) ActionValue)) false false)))

(event `EnhancedInput|/Game/Inputs/Movements/IA_LeftRight`
  (params (ActionValue :type "Float (double-precision)") (ElapsedSeconds :type "Float (double-precision)") (TriggeredSeconds :type "Float (double-precision)") (InputAction :type "InputAction Object Reference" :default "/Game/Inputs/Movements/IA_LeftRight.IA_LeftRight"))
  (bind _as_c_cam (`self.As C Cam`))
  ;[0.01896 0 1 0.5] Movement
  (:`Triggered`
    (`self.K2_AddActorLocalOffset` _as_c_cam (`KismetMathLibrary.MakeVector` 0.0 (* (`/Game/Player/C_Cam.CurrentSpeed` _as_c_cam) ActionValue)) false false)))

(event `EnhancedInput|/Game/Inputs/Movements/IA_Accelerate`
  (params (ActionValue :type Boolean) (ElapsedSeconds :type "Float (double-precision)") (TriggeredSeconds :type "Float (double-precision)") (InputAction :type "InputAction Object Reference" :default "/Game/Inputs/Movements/IA_Accelerate.IA_Accelerate"))
  (bind _as_c_cam (`self.As C Cam`))
  (bind _as_c_cam_2 (`self.As C Cam`))
  ;[0 0.7632 0.8906 0.5] Accelerate
  (:`Started`
    (set `/Game/Player/C_Cam.CurrentSpeed` (`/Game/Player/C_Cam.FastSpeed` _as_c_cam_2) _as_c_cam_2))
  (:`Canceled`
    (set `/Game/Player/C_Cam.CurrentSpeed` (`/Game/Player/C_Cam.BaseSpeed` _as_c_cam) _as_c_cam :!label _label))
  (:`Completed`
    (goto _label)))

(event `Key|MouseScrollUp`
  (params (Key :type "Key Structure"))
  (bind _as_c_cam (`self.As C Cam`))
  (bind _as_c_cam_2 (`self.As C Cam`))
  (bind _springarm (`/Game/Player/C_Cam.SpringArm` _as_c_cam_2))
  (bind _returnvalue (- (`SpringArmComponent.TargetArmLength` (`/Game/Player/C_Cam.SpringArm` _as_c_cam)) (`/Game/Player/C_Cam.ZoomSpeed` _as_c_cam)))
  ;[1 0 0.8466 0.5] Zoom
  (:`Pressed`
    (if (< _returnvalue (`/Game/Player/C_Cam.ZoomMin` _as_c_cam))
      (set `SpringArmComponent.TargetArmLength` (`/Game/Player/C_Cam.ZoomMin` _as_c_cam_2) _springarm)
      (else
        (set `SpringArmComponent.TargetArmLength` _returnvalue _springarm)))))

(event `Key|MouseScrollDown`
  (params (Key :type "Key Structure"))
  (bind _as_c_cam (`self.As C Cam`))
  (bind _as_c_cam_2 (`self.As C Cam`))
  (bind _springarm (`/Game/Player/C_Cam.SpringArm` _as_c_cam))
  (bind _returnvalue (+ (`SpringArmComponent.TargetArmLength` (`/Game/Player/C_Cam.SpringArm` _as_c_cam_2)) (`/Game/Player/C_Cam.ZoomSpeed` _as_c_cam_2)))
  ;[1 0 0.8466 0.5] Zoom
  (:`Pressed`
    (if (> _returnvalue (`/Game/Player/C_Cam.ZoomMax` _as_c_cam_2))
      (set `SpringArmComponent.TargetArmLength` (`/Game/Player/C_Cam.ZoomMax` _as_c_cam) _springarm)
      (else
        (set `SpringArmComponent.TargetArmLength` _returnvalue _springarm)))))

(fn `UserConstructionScript`)